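; Player_BP is the player character Blueprint for Demi_baby, turning input into movement, look, sprint, crouch and jump.
; Movement axes follow control-rotation yaw only, look axes drive controller pitch and yaw, and sprint swaps max walk speed while held.
; Crouch and jump block each other through IsCrouched and Jumping flags.
; Jumping clears on button release rather than landing, which only sets a separate Landed flag.
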(event `InputAxis|Forward_Back`
  (params (AxisValue :type "Float (single-precision)"))
  ;[1 1 1] Axis movement
  (`self.AddMovementInput` (`KismetMathLibrary.GetForwardVector` (`KismetMathLibrary.MakeRotator` 0.0 0.0 (.yaw (`self.GetControlRotation`)))) AxisValue))

(event `InputAxis|Right_Left`
  (params (AxisValue :type "Float (single-precision)"))
  ;[1 1 1] Axis movement
  (`self.AddMovementInput` (`KismetMathLibrary.GetRightVector` (`KismetMathLibrary.MakeRotator` 0.0 0.0 (.yaw (`self.GetControlRotation`)))) AxisValue))

(event `InputAction|Sprint`
  (params (Key :type "Key Structure"))
  (bind _charactermovement (`self.CharacterMovement`))
  ;[1 1 1] Sprint
  (:`Pressed`
    (set `CharacterMovementComponent.MaxWalkSpeed` 600.0 _charactermovement))
  (:`Released`
    (set `CharacterMovementComponent.MaxWalkSpeed` 200.0 _charactermovement)))

(event `InputAxis|Look_UpDown`
  (params (AxisValue :type "Float (single-precision)"))
  ;[1 1 1] Look with mouse or gamepad
  (`self.AddControllerPitchInput` AxisValue))

(event `InputAction|Crouch`
  (params (Key :type "Key Structure"))
  (bind _jumping (`self.Jumping`))
  ;[1 1 1] Crouch
  (:`Pressed`
    (if (not _jumping)
      (`self.Crouch`)
      (set `self.Is Crouched` true)))
  (:`Released`
    (if (not _jumping)
      (`self.UnCrouch`)
      (set `self.Is Crouched` false))))

(event `InputAxis|Look_RightLeft`
  (params (AxisValue :type "Float (single-precision)"))
  ;[1 1 1] Look with mouse or gamepad
  (`self.AddControllerYawInput` AxisValue))

(event `InputAction|Jump`
  (params (Key :type "Key Structure"))
  (bind _is_crouched (`self.Is Crouched`))
  ;[1 1 1] Jumping
  (:`Pressed`
    (if (not _is_crouched)
      (`self.Jump`)
      (set `self.Jumping` true)
      (set `self.Landed` false)))
  (:`Released`
    (if (not _is_crouched)
      (`self.StopJumping`)
      (set `self.Jumping` false))))

(event `self.OnLanded`
  (params (Hit :type "HitResult Structure (by ref)"))
  ;[1 1 1] Jumping
  (set `self.Landed` true))

(fn `UserConstructionScript`)